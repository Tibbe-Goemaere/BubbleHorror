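; BP_DoorRight is a swinging door that opens automatically on overlap with its trigger and closes when that overlap ends.
; OpenDoorCollision sets StartOpening, which Tick reads to yaw the Door at frame-rate-independent OpenSpeed toward DoorOpenRotation or back toward zero.
; A second volume, PlayerOverlapBack, sets StopMovingBack to pause opening while overlapped, but does not affect closing.
; Rotation is applied locally while the limits are checked against world yaw.
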(event OnComponentBeginOverlap(OpenDoorCollision)
  (params (OverlappedComponent :type Primitive%20Component%20Object%20Reference) (OtherActor :type Actor%20Object%20Reference) (OtherComp :type Primitive%20Component%20Object%20Reference) (OtherBodyIndex :type Integer) (bFromSweep :type Boolean) (SweepResult :type Hit%20Result%20Structure%20%28by%20ref%29))
  ;[1 1 1] Open Door
  (Variables|Default|SetStartOpening true))

(event OnComponentEndOverlap(OpenDoorCollision)
  (params (OverlappedComponent :type Primitive%20Component%20Object%20Reference) (OtherActor :type Actor%20Object%20Reference) (OtherComp :type Primitive%20Component%20Object%20Reference) (OtherBodyIndex :type Integer))
  ;[1 1 1] Close Door
  (Variables|Default|SetStartOpening false))

(event OnComponentBeginOverlap(PlayerOverlapBack)
  (params (OverlappedComponent :type Primitive%20Component%20Object%20Reference) (OtherActor :type Actor%20Object%20Reference) (OtherComp :type Primitive%20Component%20Object%20Reference) (OtherBodyIndex :type Integer) (bFromSweep :type Boolean) (SweepResult :type Hit%20Result%20Structure%20%28by%20ref%29))
  (Variables|Default|SetStopMovingBack true))

(event OnComponentEndOverlap(PlayerOverlapBack)
  (params (OverlappedComponent :type Primitive%20Component%20Object%20Reference) (OtherActor :type Actor%20Object%20Reference) (OtherComp :type Primitive%20Component%20Object%20Reference) (OtherBodyIndex :type Integer))
  (Variables|Default|SetStopMovingBack false))

(event EventBeginPlay)

(event Collision|EventActorBeginOverlap
  (params (OtherActor :type Actor%20Object%20Reference)))

(event EventTick
  (params (DeltaSeconds :type Float%20%28single-precision%29))
  (if (Variables|Default|GetStartOpening)
    (if (not (or (Variables|Default|GetStopMovingBack) (>= (.yaw (Transformation|GetWorldRotation (Variables|Default|GetDoor))) (Variables|Default|GetDoorOpenRotation))))
      (Transformation|AddLocalRotation (Variables|Default|GetDoor) (Math|Rotator|MakeRotator 0.0 0.0 (* (Variables|Default|GetOpenSpeed) DeltaSeconds)) false false))
    (elif (not (<= (.yaw (Transformation|GetWorldRotation (Variables|Default|GetDoor))) 0.0))
      (Transformation|AddLocalRotation (Variables|Default|GetDoor) (Math|Rotator|MakeRotator 0.0 0.0 (* (* (Variables|Default|GetOpenSpeed) DeltaSeconds) -1.0)) false false))))

(fn ConstructionScript)