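; BP_DoorLeftClosed is a hinged door that swings in response to the first-person character entering its trigger volumes.
; The open trigger sets StartOpening with a sound, while the close trigger clears it once through DoOnce, plays a sound and overrides OpenSpeed.
; Tick reads that flag to yaw the door in opposite directions, frame-rate independently, gated by rotation limits and StopMovingBack.
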(event OnComponentBeginOverlap(OpenDoorCollision)
  (params (OverlappedComponent :type Primitive%20Component%20Object%20Reference) (OtherActor :type Actor%20Object%20Reference) (OtherComp :type Primitive%20Component%20Object%20Reference) (OtherBodyIndex :type Integer) (bFromSweep :type Boolean) (SweepResult :type Hit%20Result%20Structure%20%28by%20ref%29))
  ;[1 1 1] Open Door
  (Utilities|Casting|CastToBP_FirstPersonCharacter OtherActor)
  (if (not (Variables|Default|GetStartOpening))
    (Audio|SpawnSoundatLocation "/Game/Sounds/DoorOpen.DoorOpen" (Transformation|GetActorLocation) "0, 0, 0" 1.0 1.0 0.0 0 0)
    (Variables|Default|SetStartOpening true)))

(event OnComponentBeginOverlap(CloseDoorCollision)
  (params (OverlappedComponent :type Primitive%20Component%20Object%20Reference) (OtherActor :type Actor%20Object%20Reference) (OtherComp :type Primitive%20Component%20Object%20Reference) (OtherBodyIndex :type Integer) (bFromSweep :type Boolean) (SweepResult :type Hit%20Result%20Structure%20%28by%20ref%29))
  (Utilities|Casting|CastToBP_FirstPersonCharacter OtherActor)
  (Utilities|FlowControl|DoOnce false
    (:Completed
      (Variables|Default|SetStartOpening false)
      (Audio|PlaySoundatLocation "/Game/Sounds/DoorClose.DoorClose" (Transformation|GetActorLocation) "0, 0, 0" 1.0 1.0 0.0 0 0 0 0)
      (Variables|Default|SetOpenSpeed 2e+02))))

(event EventBeginPlay)

(event Collision|EventActorBeginOverlap
  (params (OtherActor :type Actor%20Object%20Reference)))

(event EventTick
  (params (DeltaSeconds :type Float%20%28single-precision%29))
  (if (Variables|Default|GetStartOpening)
    (if (not (or (Variables|Default|GetStopMovingBack) (<= (Math|Float|Absolute(Float) (.yaw (.rotation (Transformation|GetRelativeTransform (Variables|Default|GetDoor))))) (Math|Float|Absolute(Float) (Variables|Default|GetDoorOpenRotation)))))
      (Transformation|AddLocalRotation (Variables|Default|GetDoor) (Math|Rotator|MakeRotator 0.0 0.0 (* (Variables|Default|GetOpenSpeed) DeltaSeconds)) false false))
    (elif (not (>= (.yaw (.rotation (Transformation|GetRelativeTransform (Variables|Default|GetDoor)))) 0.0))
      (Transformation|AddLocalRotation (Variables|Default|GetDoor) (Math|Rotator|MakeRotator 0.0 0.0 (* (* (Variables|Default|GetOpenSpeed) DeltaSeconds) -1.0)) false false))))

(fn ConstructionScript)